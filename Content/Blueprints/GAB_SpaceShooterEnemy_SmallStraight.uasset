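; Small space shooter enemy that flies straight along its local Y axis at a set speed, using a swept offset each Tick.
; Overlapping a player projectile destroys both actors, while overlapping the shield destroys only the enemy.
; Either kill spawns an explosion and sound, then reports points to the player's HUD.
; A separate Destroy event plays the same effects and removes the enemy without awarding score.
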(event `self.ReceiveTick`
  (params (DeltaSeconds :type "Float (single-precision)"))
  (`self.K2_AddActorLocalOffset` (`KismetMathLibrary.MakeVector` 0.0 (* DeltaSeconds (`self.Speed`))) true))

(event `self.ReceiveActorBeginOverlap`
  (params (OtherActor :type "Actor Object Reference"))
  (bind _returnvalue (`GameplayStatics.GetObjectClass` OtherActor))
  (if (== _returnvalue "/Game/Blueprints/GAB_SpaceShooterPlayerProj01.GAB_SpaceShooterPlayerProj01_C")
    (`self.K2_DestroyActor` OtherActor :!label _label)
    (`GameplayStatics.SpawnEmitterAtLocation` "/Game/Particles/P_Explosion.P_Explosion" (`self.K2_GetActorLocation`) :!label _label_2)
    (`GameplayStatics.PlaySoundAtLocation` "/Game/Audio/Sounds/EnemySmallDestroyed.EnemySmallDestroyed" (0.0 0.0 0.0) 1.0 1.0)
    (`self.K2_DestroyActor`)
    (message `/Game/Blueprints/GAB_SpaceShooterBlueprintInterfacesBlue.EnemyDestroyedUpdateScore` (`PlayerController.GetHUD` (`GameplayStatics.GetPlayerController` 0)) 150)
    (elif (== _returnvalue "/Game/Blueprints/GAB_SpaceShooterPlayerProj02.GAB_SpaceShooterPlayerProj02_C")
      (goto _label)
      (elif (== _returnvalue "/Game/Blueprints/GAB_SpaceShooterPlayerProj03.GAB_SpaceShooterPlayerProj03_C")
        (goto _label)
        (elif (== _returnvalue "/Game/Blueprints/GAB_SpaceShooterPlayerProj04.GAB_SpaceShooterPlayerProj04_C")
          (goto _label)
          (elif (== _returnvalue "/Game/Blueprints/GAB_SpaceShooterShield.GAB_SpaceShooterShield_C")
            (goto _label_2)))))))

(event `Destroy`
  (`GameplayStatics.SpawnEmitterAtLocation` "/Game/Particles/P_Explosion.P_Explosion" (`self.K2_GetActorLocation`))
  (`GameplayStatics.PlaySoundAtLocation` "/Game/Audio/Sounds/EnemySmallDestroyed.EnemySmallDestroyed" (0.0 0.0 0.0) 1.0 1.0)
  (`self.K2_DestroyActor`))

(fn `UserConstructionScript`
  (`parent.UserConstructionScript`))