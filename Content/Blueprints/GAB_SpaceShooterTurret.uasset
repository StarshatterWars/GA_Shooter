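; Enemy turret for a space shooter that wakes once its Y offset from the player drops below 600, then stays active.
; While active, Tick turns it toward the player with a yaw offset, and a DoOnce starts a Delay loop firing a projectile every second.
; Overlapping player projectiles are destroyed and drain Health; a hit at zero, or any shield contact, explodes the turret and reports score to the HUD.
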(event `self.ReceiveTick`
  (params (DeltaSeconds :type "Float (single-precision)"))
  (bind _returnvalue (`self.K2_GetActorLocation`))
  (bind _returnvalue_2 (`self.K2_GetActorLocation` (`GameplayStatics.GetPlayerPawn` 0)))
  (if (< (.y (- _returnvalue _returnvalue_2)) 600.0)
    (set `self.Active` true))
  (if (`self.Active`)
    (`self.SetActorRotation` (`KismetMathLibrary.MakeRot` (.pitch (`KismetMathLibrary.FindLookAtRotation` _returnvalue _returnvalue_2)) (+ (.yaw (`KismetMathLibrary.FindLookAtRotation` _returnvalue _returnvalue_2)) 90.0) (.roll (`KismetMathLibrary.FindLookAtRotation` _returnvalue _returnvalue_2))))
    (`/Engine/EditorBlueprintResources/StandardMacros.DoOnce` false
      (:`Completed`
        (`|SpawnActorFromClass` "/Game/Blueprints/GAB_SpaceShooterTurretProj.GAB_SpaceShooterTurretProj_C" (`self.GetTransform`) :!label _label)
        (`GameplayStatics.PlaySoundAtLocation` "/Game/Audio/Sounds/TurretShooting.TurretShooting" (0.0 0.0 0.0) 1.0 1.0)
        (`KismetSystemLibrary.Delay` 1.0)
        (goto _label)))))

(event `self.ReceiveActorBeginOverlap`
  (params (OtherActor :type "Actor Object Reference"))
  (bind _returnvalue (`GameplayStatics.GetObjectClass` OtherActor))
  (if (== _returnvalue "/Game/Blueprints/GAB_SpaceShooterPlayerProj01.GAB_SpaceShooterPlayerProj01_C")
    (`self.K2_DestroyActor` OtherActor :!label _label_2)
    (if (> (`self.Health`) 0)
      (set `self.Health` (- (`self.Health`) 1))
      (`GameplayStatics.PlaySoundAtLocation` "/Game/Audio/Sounds/TurretImpact.TurretImpact" (0.0 0.0 0.0) 1.0 1.0)
      (else
        (`GameplayStatics.SpawnEmitterAtLocation` "/Game/Particles/P_Explosion.P_Explosion" (`self.K2_GetActorLocation`) :!label _label_3)
        (`GameplayStatics.PlaySoundAtLocation` "/Game/Audio/Sounds/TurretDestroyed.TurretDestroyed" (0.0 0.0 0.0) 1.0 1.0)
        (`self.K2_DestroyActor`)
        (message `/Game/Blueprints/GAB_SpaceShooterBlueprintInterfacesBlue.EnemyDestroyedUpdateScore` (`PlayerController.GetHUD` (`GameplayStatics.GetPlayerController` 0)) 100)))
    (elif (== _returnvalue "/Game/Blueprints/GAB_SpaceShooterPlayerProj02.GAB_SpaceShooterPlayerProj02_C")
      (goto _label_2)
      (elif (== _returnvalue "/Game/Blueprints/GAB_SpaceShooterPlayerProj03.GAB_SpaceShooterPlayerProj03_C")
        (goto _label_2)
        (elif (== _returnvalue "/Game/Blueprints/GAB_SpaceShooterPlayerProj04.GAB_SpaceShooterPlayerProj04_C")
          (goto _label_2)
          (elif (== _returnvalue "/Game/Blueprints/GAB_SpaceShooterShield.GAB_SpaceShooterShield_C")
            (goto _label_3)))))))

(fn `UserConstructionScript`)